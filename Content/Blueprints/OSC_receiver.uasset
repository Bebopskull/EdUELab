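; OSC receiver actor that listens for Open Sound Control messages over the network and prints them for debugging.
; On BeginPlay it creates and stores an OSC server on a hardcoded local IP and port, clears bundle-received bindings and binds a message-received handler.
; The handler prints each message's full address path and the sender's IP, without reading the message's values.
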(event Custom|CustomEvent_0
  (params (Message :type OSC%20Message%20Structure%20%28by%20ref%29) (IPAddress :type String) (Port :type Integer))
  (Utilities|FlowControl|Sequence
    (:then_0
      (bind _returnvalue (Class|OSCManager|GetOSCMessageAddress Message))
      (bind _returnvalue_2 (Class|OSCManager|GetOSCAddressFullPath _returnvalue))
      (Development|PrintString _returnvalue_2))
    (:then_1
      (Development|PrintString IPAddress))))

(event EventBeginPlay
  (bind _returnvalue (Class|OSCManager|CreateOSCServer "192.168.2.10" 7000 false false "" 0))
  (bind _output_get (Variables|Default|SetOSCdata _returnvalue))
  (EventDispatchers|UnbindallEventsfromOnOscBundleReceived _output_get)
  (EventDispatchers|BindEventtoOnOscMessageReceived _output_get (EventDispatchers|CreateEvent :!event Custom|CustomEvent_0)))

(fn ConstructionScript)