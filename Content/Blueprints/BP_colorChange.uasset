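; BP_colorChange is an actor that cycles a point light's color through a list when Enter is pressed.
; A custom CycleCOlor event sets the PointLight color from ColorList at the current Index.
; Each press applies that color, then advances Index, wrapping back to zero after the last entry.
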(event Custom|CycleCOlor
  ;[1 1 1] CycleColor Function
  (Rendering|Components|Light|SetLightColor (Variables|Default|GetPointLight) (Utilities|Array|Get(acopy) (Variables|Default|GetColorList) (Variables|Default|GetIndex)) true))

(event EventBeginPlay)

(event Collision|EventActorBeginOverlap
  (params (OtherActor :type Actor%20Object%20Reference)))

(event EventTick
  (params (DeltaSeconds :type Float%20%28single-precision%29)))

(event Input|KeyboardEvents|Enter
  (params (Key :type Key%20Structure :default "None"))
  ;[1 1 1] CycleColor Function Execution and workflow
  (:Pressed
    (CallFunction|CycleCOlor)
    (if (< (Variables|Default|GetIndex) (- (Utilities|Array|Length (Variables|Default|GetColorList)) 1))
      (Math|Integer|IncrementInt (Variables|Default|GetIndex))
      (else
        (Variables|Default|SetIndex 0)))))

(fn ConstructionScript)