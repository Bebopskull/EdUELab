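; BP_TDEX is a Blueprint that drives a flickering spotlight with a key-switched color.
; Each Tick samples 1D Perlin noise from game time scaled by Speed, then remaps it to a light intensity capped by MaxFlickerIntensity.
; Any key press advances a looping, sequential MultiGate that cycles the light through blue, pink, yellow and near-white.
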(event EventBeginPlay)

(event EventTick
  (params (DeltaSeconds :type Float%20%28single-precision%29))
  ;[1 1 1] Generate perlin noise flicker for light intensity
  (Rendering|Components|Light|SetIntensity (Variables|Default|GetSpotLight) (Math|Float|MapRangeClamped (Class|KismetMathLibrary|PerlinNoise1D (* (Utilities|Time|GetGameTimeinSeconds) (Variables|Default|GetSpeed))) -1.0 1.0 0.0 (Variables|Default|GetMax%20flicker%20Intensity))))

(event Input|KeyboardEvents|AnyKey
  (params (Key :type Key%20Structure :default "None"))
  (bind _spotlight (Variables|Default|GetSpotLight))
  ;[1 1 1] Color cycle
  (:Pressed
    (Utilities|FlowControl|MultiGate false true 0
      (:Out%200
        (Rendering|Components|Light|SetLightColor _spotlight "(R=0.000000,G=0.077639,B=1.000000,A=1.000000)" true))
      (:Out%201
        (Rendering|Components|Light|SetLightColor _spotlight "(R=1.000000,G=0.000000,B=0.394844,A=1.000000)" true))
      (:Out%202
        (Rendering|Components|Light|SetLightColor _spotlight "(R=0.930075,G=1.000000,B=0.000000,A=1.000000)" true))
      (:Out%203
        (Rendering|Components|Light|SetLightColor _spotlight "(R=0.998667,G=0.976708,B=1.000000,A=1.000000)" true)))))

(fn ConstructionScript)