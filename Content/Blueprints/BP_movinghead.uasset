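; Moving-head spotlight fixture with a yoke that pans on yaw and a head pivot that tilts on inverted roll.
; The construction script applies the X and Y angles to the pivots and sets the spotlight's color and intensity.
; When Autoanimate is on, Tick overrides both rotations using Perlin noise over game time scaled by Speed.
; Pan and tilt share the same noise input, so their motion is correlated.
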(event EventBeginPlay)

(event Collision|EventActorBeginOverlap
  (params (OtherActor :type Actor%20Object%20Reference)))

(event EventTick
  (params (DeltaSeconds :type Float%20%28single-precision%29))
  (bind _returnvalue (Utilities|Time|GetGameTimeinSeconds))
  (bind _speed (Variables|Default|GetSpeed))
  (bind _returnvalue_2 (* _returnvalue _speed))
  (if (Variables|Default|GetAutoanimate)
    (Transformation|SetRelativeRotation (Variables|Default|GetMover_Yoke) (Math|Rotator|MakeRotator 0.0 0.0 (Math|Float|MapRangeClamped (Class|KismetMathLibrary|PerlinNoise1D _returnvalue_2) -1.0 1.0 0.0 3.6e+02)) false false)
    (Transformation|SetRelativeRotation (Variables|Default|GetHeadPivot) (Math|Rotator|MakeRotator (* (Math|Float|MapRangeClamped (Class|KismetMathLibrary|PerlinNoise1D _returnvalue_2) -1.0 1.0 -9e+01 1.8e+02) -1.0) 0.0 0.0) false false)))

(fn ConstructionScript
  (bind _spotlight (Variables|Default|GetSpotLight))
  (Transformation|SetRelativeRotation (Variables|Default|GetMover_Yoke) (Math|Rotator|MakeRotator 0.0 0.0 (Variables|Default|GetX)) false false)
  (Transformation|SetRelativeRotation (Variables|Default|GetHeadPivot) (Math|Rotator|MakeRotator (* (Variables|Default|GetY) -1.0) 0.0 0.0) false false)
  (Rendering|Components|Light|SetLightColor _spotlight (Variables|Default|GetNew%20Light%20Color) true)
  (Rendering|Components|Light|SetIntensity _spotlight (Variables|Default|GetNew%20Intensity)))