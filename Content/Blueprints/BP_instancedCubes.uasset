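; Actor that displays a grid of instanced cubes in the YZ plane, animated to oscillate along X.
; The construction script builds the grid from Columns, Rows and Spacing, scales instances by Spacing and caches transforms in PosArray with unit scale.
; A Tick counter feeds a per-index sine offset that Timeline updates apply to every instance, also replacing the constructed scale with the cached one.
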(event EventBeginPlay
  (bind _posarray (Variables|Default|GetPosArray))
  ;[1 1 1] Anim
  (bind _lfo (Timeline|Timeline_0 Play)
    (:Update
      (for _index (range 0 (- (Utilities|Array|Length _posarray) 1))
        (Components|InstancedStaticMesh|UpdateInstanceTransform (Variables|Default|GetInstancedStaticMesh) _index (Math|Transform|MakeTransform (Math|Vector|MakeVector (* (+ (Math|Trig|Sin(Degrees) (* (/ (Math|Conversions|ToFloat(Integer) (stale EventTick _output_get)) 1.0) (Math|Trig|Cos(Radians) (Math|Conversions|ToFloat(Integer) _index)))) (.x (.location (Utilities|Array|Get(acopy) _posarray _index)))) 2e+01) (.y (.location (Utilities|Array|Get(acopy) _posarray _index))) (.z (.location (Utilities|Array|Get(acopy) _posarray _index)))) (.rotation (Utilities|Array|Get(acopy) _posarray _index)) (.scale (Utilities|Array|Get(acopy) _posarray _index))) false true false)))))

(event Collision|EventActorBeginOverlap
  (params (OtherActor :type Actor%20Object%20Reference)))

(event EventTick
  (params (DeltaSeconds :type Float%20%28single-precision%29))
  ;[1 1 1] Anim
  (bind _output_get (Variables|Default|Settime (+ (Variables|Default|Gettime) 1))))

(fn ConstructionScript
  (bind _spacing (Variables|Default|Getspacing))
  (bind _columns (Variables|Default|GetColumns))
  (bind _returnvalue (Math|Float|Division(WholeandRemainder) _spacing 1e+02))
  (bind _returnvalue_2 (Math|Conversions|ToFloat(Integer) _returnvalue))
  ;[1 1 1] Construction
  (for _index (range 0 _columns)
    (for _index_2 (range 0 (Variables|Default|GetRows))
      (Components|InstancedStaticMesh|AddInstance (Variables|Default|GetInstancedStaticMesh) (Math|Transform|MakeTransform (Math|Vector|MakeVector 0.0 (- (* _index _spacing) (* _spacing (/ (Math|Conversions|ToFloat(Integer) _columns) 2.0))) (- (* _index_2 _spacing) _spacing)) "0, 0, 0" (Math|Vector|MakeVector _returnvalue_2 _returnvalue_2 _returnvalue_2)))
      (Utilities|Array|Add (Variables|Default|GetPosArray) (Math|Transform|MakeTransform (Math|Vector|MakeVector 0.0 (.Y (Math|Vector|BreakVector (Math|Vector|MakeVector 0.0 (- (* _index _spacing) (* _spacing (/ (Math|Conversions|ToFloat(Integer) _columns) 2.0))) (- (* _index_2 _spacing) _spacing)))) (.Z (Math|Vector|BreakVector (Math|Vector|MakeVector 0.0 (- (* _index _spacing) (* _spacing (/ (Math|Conversions|ToFloat(Integer) _columns) 2.0))) (- (* _index_2 _spacing) _spacing))))) "0, 0, 0" "1,1,1")))))